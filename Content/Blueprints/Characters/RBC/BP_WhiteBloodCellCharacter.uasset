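; Player character Blueprint for the white blood cell.
; On BeginPlay it spawns a BP_CameraManager at its location with itself as the follow target, then makes that the player controller's view target.
; A disconnected, debug-drawn prototype intersects the cursor ray with the character's Y-normal plane and traces to it from the Head socket; its note says this logic has moved to C++.
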(event EventBeginPlay
  (bind _returnvalue (Game|SpawnActorfromClass "/Game/Blueprints/Characters/WBC/BP_CameraManager.BP_CameraManager_C" (Math|Transform|MakeTransform (Transformation|GetActorLocation) "0, 0, 0" "1.000000,1.000000,1.000000") "Undefined" "MultiplyWithRoot" 0 self 0))
  (Game|Player|SetViewTargetwithBlend (Game|GetPlayerController 0) _returnvalue 0.0 "VTBlend_Linear" 0.0 false))

(event Collision|EventActorBeginOverlap
  (params (OtherActor :type Actor%20Object%20Reference)))

(event EventTick
  (params (DeltaSeconds :type Float%20%28single-precision%29)))

(fn ConstructionScript)