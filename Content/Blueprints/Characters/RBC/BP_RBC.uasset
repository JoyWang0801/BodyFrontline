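; BP_RBC is an RBC character that dissolves visually when it dies.
; The RBCDie event creates a dynamic M_Dissolve material on the mesh and steps its Dissolve parameter down from DissolveConstant in a delayed loop.
; Once the threshold is reached it destroys the actor, with no respawn logic here despite the "Die and respawn" label.
; BeginPlay only prints the actor's location.
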(event EventBeginPlay
  (Development|PrintString (Utilities|String|ToString(Vector) (Transformation|GetActorLocation))))

(event Collision|EventActorBeginOverlap
  (params (OtherActor :type Actor%20Object%20Reference)))

(event EventTick
  (params (DeltaSeconds :type Float%20%28single-precision%29)))

(event EventRBCDie
  ;[1 1 1] Die and respawn
  (bind _returnvalue (Rendering|Material|CreateDynamicMaterialInstance (Variables|Character|GetMesh) 0 "/Game/Assets/fx/M_Dissolve.M_Dissolve" "None" :!class /Script/Engine.PrimitiveComponent))
  (if (> (Variables|Default|GetDissolveConstant) -0.5) :!label _label
    (Rendering|Material|SetScalarParameterValue _returnvalue "Dissolve" (Variables|Default|GetDissolveConstant) :!class /Script/Engine.MaterialInstanceDynamic)
    (Rendering|Material|SetMaterial (Variables|Character|GetMesh) 0 _returnvalue)
    (Variables|Default|SetDissolveConstant (- (Variables|Default|GetDissolveConstant) 0.3))
    (Utilities|FlowControl|Delay 0.05)
    (goto _label)
    (else
      (Actor|DestroyActor))))

(fn ConstructionScript)