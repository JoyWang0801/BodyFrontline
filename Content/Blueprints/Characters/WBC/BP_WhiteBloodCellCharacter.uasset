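; Player white blood cell character Blueprint, handling camera setup and death respawn.
; On BeginPlay it spawns a BP_CameraManager that follows it and makes that the view target.
; When Dead, PlayDeathMaterial steps a dynamic M_Dissolve material down in a Delay loop, then moves the cell beside the "Base"-tagged actor and resets only the dissolve variable.
; An unused cursor plane-intersection trace remains, noted as migrated to C++.
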(event EventBeginPlay
  (bind _returnvalue (Game|SpawnActorfromClass "/Game/Blueprints/Characters/WBC/BP_CameraManager.BP_CameraManager_C" (Math|Transform|MakeTransform (Transformation|GetActorLocation) "0, 0, 0" "1.000000,1.000000,1.000000") "Undefined" "MultiplyWithRoot" 0 self 0))
  (Game|Player|SetViewTargetwithBlend (Game|GetPlayerController 0) _returnvalue 0.0 "VTBlend_Linear" 0.0 false))

(event Collision|EventActorBeginOverlap
  (params (OtherActor :type Actor%20Object%20Reference)))

(event EventTick
  (params (DeltaSeconds :type Float%20%28single-precision%29)))

(event EventPlayDeathMaterial
  ;[1 1 1] Die and respawn
  (if (Utilities|Enum|Equal(Enum) (Variables|Default|GetWBCState) "ECS_Dead")
    (bind _returnvalue (Rendering|Material|CreateDynamicMaterialInstance (Variables|Character|GetMesh) 0 "/Game/Assets/fx/Dissolve/M_Dissolve.M_Dissolve" "None" :!class /Script/Engine.PrimitiveComponent))
    (if (> (Variables|Default|GetDissolveConstant) -0.5) :!label _label
      (Rendering|Material|SetScalarParameterValue _returnvalue "Dissolve" (Variables|Default|GetDissolveConstant) :!class /Script/Engine.MaterialInstanceDynamic)
      (Rendering|Material|SetMaterial (Variables|Character|GetMesh) 0 _returnvalue)
      (Variables|Default|SetDissolveConstant (- (Variables|Default|GetDissolveConstant) 0.2))
      (Utilities|FlowControl|Delay 0.1)
      (goto _label)
      (else
        (bind _outactors (Actor|GetAllActorswithTag "Base"))
        (Transformation|SetActorLocation (Math|Vector|MakeVector (+ 1e+02 (.x (Transformation|GetActorLocation (Utilities|Array|Get(acopy) _outactors)))) (.y (Transformation|GetActorLocation (Utilities|Array|Get(acopy) _outactors))) (.z (Transformation|GetActorLocation (Utilities|Array|Get(acopy) _outactors)))) false false)
        (Variables|Default|SetDissolveConstant 1.0)))))

(fn ConstructionScript)