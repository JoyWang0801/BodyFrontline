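; BP_CameraManager is a camera-manager actor that smoothly follows FollowTarget.
; Every Tick, UpdateCameraPos moves the actor with VInterpTo at Speed toward the target's location, pushed along its forward vector by CamOffset.
; The offset applies only on X and Z, leaving Y on the target.
; LockHeight swaps the target's Z for the actor's current Z before the offset is added.
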(event EventBeginPlay)

(event Collision|EventActorBeginOverlap
  (params (OtherActor :type Actor%20Object%20Reference)))

(event EventTick
  (params (DeltaSeconds :type Float%20%28single-precision%29))
  (CallFunction|UpdateCameraPos))

(fn ConstructionScript)

(fn UpdateCameraPos
  (bind _followtarget (Variables|Default|GetFollowTarget))
  (bind _followtarget_2 (Variables|Default|GetFollowTarget))
  (bind _camoffset (LocalVariables|GetCamOffset))
  (bind _returnvalue (Transformation|GetActorForwardVector _followtarget_2))
  (bind _returnvalue_2 (Transformation|GetActorLocation _followtarget))
  (bind _returnvalue_3 (* _returnvalue _camoffset))
  (Transformation|SetActorLocation (Math|Interpolation|VInterpTo (Transformation|GetActorLocation) (+ (Math|Vector|MakeVector (.x _returnvalue_2) (.y _returnvalue_2) (select (LocalVariables|GetLockHeight) (.z (Transformation|GetActorLocation)) (.z _returnvalue_2))) (Math|Vector|MakeVector (.x _returnvalue_3) 0.0 (.z _returnvalue_3))) (Utilities|Time|GetWorldDeltaSeconds) (LocalVariables|GetSpeed)) false false))