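; BP_Base is the base actor in Body Frontline, acting as an AI director that periodically redistributes all BP_Enemy targets.
; A looping timer sizes base, RBC and player quotas from enemy count and game difficulty, weighted up as base health, RBC count or player health drops.
; Enemy states are filled in base, RBC, player order, leaving any surplus enemies unchanged.
; Debug prints show each quota and running totals that never reset.
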(event Custom|DirectorAI
  (bind _outactors (Actor|GetAllActorsOfClass "/Game/Blueprints/Enemy/BP_Enemy.BP_Enemy_C"))
  (CallFunction|CalculateDistribution _outactors)
  (for (_ _array_index) _outactors
    (if (== (Variables|Default|GetTargetingBase) 0)
      (if (== (Variables|Default|GetTargetingRBC) 0)
        (if (not (== (Variables|Default|GetTargetingPlayer) 0))
          (if (Utilities|Enum|Equal(Enum) (Variables|/Script/BodyFrontline.Enemy|GetEnemyState (Utilities|Array|Get(acopy) _outactors _array_index)) "EVS_Chasing_Player")
            _
            (else
              (Variables|/Script/BodyFrontline.Enemy|SetEnemyState (Utilities|Array|Get(acopy) _outactors _array_index) "EVS_Chasing_Player")))
          (Variables|Default|SetTargetingPlayer (- (Variables|Default|GetTargetingPlayer) 1))
          (Variables|Default|SetTotalTargetingPlayer (+ (Variables|Default|GetTotalTargetingPlayer) 1)))
        (else
          (if (Utilities|Enum|Equal(Enum) (Variables|/Script/BodyFrontline.Enemy|GetEnemyState (Utilities|Array|Get(acopy) _outactors _array_index)) "EVS_Attacking_RBC")
            _
            (else
              (Variables|/Script/BodyFrontline.Enemy|SetEnemyState (Utilities|Array|Get(acopy) _outactors _array_index) "EVS_Attacking_RBC")))
          (Variables|Default|SetTargetingRBC (- (Variables|Default|GetTargetingRBC) 1))
          (Variables|Default|SetTotalTargetingRBC (+ (Variables|Default|GetTotalTargetingRBC) 1))))
      (else
        (if (Utilities|Enum|Equal(Enum) (Variables|/Script/BodyFrontline.Enemy|GetEnemyState (Utilities|Array|Get(acopy) _outactors _array_index)) "EVS_Attacking_Base")
          _
          (else
            (Variables|/Script/BodyFrontline.Enemy|SetEnemyState (Utilities|Array|Get(acopy) _outactors _array_index) "EVS_Attacking_Base")))
        (Variables|Default|SetTargetingBase (- (Variables|Default|GetTargetingBase) 1))
        (Variables|Default|SetTotalTargetingBase (+ (Variables|Default|GetTotalTargetingBase) 1)))))
  (Development|PrintString (Utilities|String|Append "Total Targeting Base : " (Utilities|String|ToString(Integer) (Variables|Default|GetTotalTargetingBase))) true true "(R=0.604167,G=0.208333,B=1.000000,A=1.000000)" 1e+01)
  (Development|PrintString (Utilities|String|Append "Total Targeting Player : " (Utilities|String|ToString(Integer) (Variables|Default|GetTotalTargetingPlayer))) true true "(R=0.604167,G=0.208333,B=1.000000,A=1.000000)" 1e+01)
  (Development|PrintString (Utilities|String|Append "Total Targeting RBC : " (Utilities|String|ToString(Integer) (Variables|Default|GetTotalTargetingRBC))) true true "(R=0.604167,G=0.208333,B=1.000000,A=1.000000)" 1e+01))

(event EventBeginPlay
  (Utilities|Time|SetTimerbyEvent (delegate Custom|DirectorAI) 1e+01 true))

(event Collision|EventActorBeginOverlap
  (params (OtherActor :type Actor%20Object%20Reference)))

(event EventTick
  (params (DeltaSeconds :type Float%20%28single-precision%29)))

(fn ConstructionScript)

(fn GetGameDifficulty
  (bind _asbp_body_friontline_game_instance (Utilities|Casting|CastToBP_BodyFriontlineGameInstance (Game|GetGameInstance)))
  (if (Utilities|Enum|Equal(Enum) (Variables|/Script/BodyFrontline.BodyFrontlineGameInstance|GetDiffculty _asbp_body_friontline_game_instance) "EGD_Easy")
    (return 0.1)
    (elif (Utilities|Enum|Equal(Enum) (Variables|/Script/BodyFrontline.BodyFrontlineGameInstance|GetDiffculty _asbp_body_friontline_game_instance) "EGD_Medium")
      (return 0.15)
      (elif (Utilities|Enum|Equal(Enum) (Variables|/Script/BodyFrontline.BodyFrontlineGameInstance|GetDiffculty _asbp_body_friontline_game_instance) "EGD_Hard")
        (return 0.2)))))

(fn CalculateDistribution
  (params (EnemyArray :type Array%20of%20BP%20Enemy%20Object%20References))
  (bind _returnvalue (Utilities|Array|Length EnemyArray))
  (bind _add_distribution (CallFunction|GetGameDifficulty))
  (bind _asbp_white_blood_cell_character (Utilities|Casting|CastToBP_WhiteBloodCellCharacter (Game|GetPlayerCharacter 0)))
  (bind _add_distribution_2 (CallFunction|GetRBClevel _asbp_white_blood_cell_character))
  (Variables|Default|SetTargetingRBC (+ (Math|Float|Round (* (+ _add_distribution _add_distribution_2) _returnvalue)) 1))
  (bind _add_distribution_3 (CallFunction|GetPlayerHealthLevel _asbp_white_blood_cell_character))
  (Variables|Default|SetTargetingPlayer (+ (Math|Float|Round (* (+ _add_distribution _add_distribution_3) _returnvalue)) 1))
  (bind _add_distribution_4 (CallFunction|GetBaseHealthLevel))
  (Variables|Default|SetTargetingBase (+ (Math|Float|Round (* (+ _add_distribution_4 _add_distribution) _returnvalue)) 1))
  (Development|PrintString (Utilities|String|Append "Added Targeting Base : " (Utilities|String|ToString(Integer) (Variables|Default|GetTargetingBase))) true true "(R=1.000000,G=0.407843,B=0.000000,A=1.000000)" 1e+01)
  (Development|PrintString (Utilities|String|Append "Added Targeting Player : " (Utilities|String|ToString(Integer) (Variables|Default|GetTargetingPlayer))) true true "(R=1.000000,G=0.407843,B=0.000000,A=1.000000)" 1e+01)
  (Development|PrintString (Utilities|String|Append "Added Targeting RBC : " (Utilities|String|ToString(Integer) (Variables|Default|GetTargetingRBC))) true true "(R=1.000000,G=0.407843,B=0.000000,A=1.000000)" 1e+01))

(fn GetRBClevel
  (params (Character :type BP%20White%20Blood%20Cell%20Character%20Object%20Reference))
  (bind _returnvalue (Class|WhiteBloodCellCharacter|RBCCount Character))
  (if (<= _returnvalue 1)
    (return 0.15) ; low
    (elif (Math|Integer|InRange(Integer) _returnvalue 2 4)
      (return 0.05) ; medium
      (elif (>= _returnvalue 5)
        (return 0.0) ; high
      ))))

(fn GetBaseHealthLevel
  (bind _returnvalue (Actor|GetActorOfClass "BP_Base_C"))
  (bind _returnvalue_2 (Class|Base|GetBaseHealth _returnvalue))
  (if (Math|Integer|InRange(Integer) _returnvalue_2 70 100)
    (return 0.0) ; high
    (elif (Math|Integer|InRange(Integer) _returnvalue_2 30 70 true false)
      (return 0.05) ; medium
      (else
        (return 0.15) ; low
      ))))

(fn GetPlayerHealthLevel
  (params (Character :type BP%20White%20Blood%20Cell%20Character%20Object%20Reference))
  (bind _returnvalue (Class|WhiteBloodCellCharacter|HealthPercent Character))
  (if (>= _returnvalue 0.75)
    (return 0.0) ; high
    (elif (Math|Float|InRange(Float) _returnvalue 0.4 0.75 false false)
      (return 0.05) ; medium
      (elif (<= _returnvalue 0.4)
        (return 0.1) ; low
      ))))