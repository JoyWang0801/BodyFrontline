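; Enemy wave spawner that spawns BP_Enemy at its own location, sizing each wave to how the player is doing.
; SpawnEnemy sums a default count with offsets from base health, difficulty, player health, wave number, RBC count and last clear time, then staggers spawns randomly.
; A looping 30-second timer drives waves; Tick detects when all enemies are gone, records clear time and restarts the timer with a negative start delay.
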(event Custom|SpawnEnemy
  (bind _returnvalue (Actor|GetActorOfClass "/Game/Blueprints/Items/BP_Base.BP_Base_C"))
  (bind _returnvalue_2 (Class|Base|GetBaseHealth _returnvalue))
  (Development|PrintString (Utilities|String|Append "Default enemy spawning amount: " (Utilities|String|ToString(Integer) (Variables|Default|GetDefault_Enemy))) true true "(R=0.000000,G=0.660000,B=1.000000,A=1.000000)" 1e+01)
  (bind _asbp_white_blood_cell_character (Utilities|Casting|CastToBP_WhiteBloodCellCharacter (Game|GetPlayerCharacter 0)))
  (bind _lastindex (CallFunction|GetBaseHealthEnemyOffset _returnvalue_2))
  (bind _difficultyoffset (CallFunction|GetGameDifficultyEnemyOffset))
  (bind _playerhealthoffset (CallFunction|GetPlayerHealthEnemyOffset _asbp_white_blood_cell_character))
  (bind _playerhealthoffset_2 (CallFunction|GetProgressEnemyOffset _asbp_white_blood_cell_character))
  (bind _playerhealthoffset_3 (CallFunction|GetRBCEnemyOffset _asbp_white_blood_cell_character))
  (bind _timeenemyoffset (CallFunction|CalculateTimeEnemyOffset (Variables|Default|GetTimeElapsed)))
  (Class|WhiteBloodCellCharacter|UpdateWaveNumber _asbp_white_blood_cell_character)
  (Variables|Default|SetnumberOfEnemy (+ _lastindex _difficultyoffset _playerhealthoffset _playerhealthoffset_2 _playerhealthoffset_3 _timeenemyoffset))
  (Development|PrintString (Utilities|String|Append "Total number of enemy spawning: " (Utilities|String|ToString(Integer) (+ _lastindex _difficultyoffset _playerhealthoffset _playerhealthoffset_2 _playerhealthoffset_3 _timeenemyoffset))) true true "(R=1.000000,G=0.080438,B=0.150141,A=1.000000)" 1e+01)
  (if (Variables|Default|GetTimerStarted)
    _
    (else
      (Variables|Default|SetStartTime (Utilities|Time|GetRealTimeSeconds))
      (Variables|Default|SetTimerStarted true)))
  (Variables|Default|SetSpawnCounter 0)
  (if (< (Variables|Default|GetSpawnCounter) (Variables|Default|GetnumberOfEnemy)) :!label _label
    (Game|SpawnActorfromClass "/Game/Blueprints/Enemy/BP_Enemy.BP_Enemy_C" (Transformation|GetActorTransform) "Undefined" "MultiplyWithRoot" 0 0)
    (Utilities|Array|Add (Variables|Default|GetEnemies) 0)
    (Variables|Default|SetSpawnCounter (+ (Variables|Default|GetSpawnCounter) 1))
    (Utilities|FlowControl|Delay (Math|Random|RandomFloatinRange 0.0 2.0))
    (goto _label)))

(event EventBeginPlay
  (bind _returnvalue (Utilities|Time|SetTimerbyEvent (delegate Custom|SpawnEnemy) 3e+01 true -3e+01))
  (Variables|Default|SetTimer _returnvalue))

(event EventTick
  (params (DeltaSeconds :type Float%20%28single-precision%29))
  (bind _outactors (Actor|GetAllActorsOfClass "/Game/Blueprints/Enemy/BP_Enemy.BP_Enemy_C"))
  (bind _output_get (Variables|Default|SetEnemies _outactors))
  (if (and (== (Utilities|Array|Length _output_get) 0) (Variables|Default|GetTimerStarted))
    (Variables|Default|SetEndTime (Utilities|Time|GetRealTimeSeconds))
    (Variables|Default|SetTimeElapsed (- (Variables|Default|GetEndTime) (Variables|Default|GetStartTime)))
    (Development|PrintString (Utilities|String|Append "It took:  " (Utilities|String|ToString(Float) (- (Variables|Default|GetEndTime) (Variables|Default|GetStartTime))) " to finish this wave") true true "(R=0.000000,G=0.660000,B=1.000000,A=1.000000)" 1e+01)
    (Variables|Default|SetTimerStarted false)
    (Utilities|Time|ClearandInvalidateTimerbyHandle (Variables|Default|GetTimer))
    (bind _returnvalue (Utilities|Time|SetTimerbyEvent (delegate Custom|SpawnEnemy) 3e+01 true -3e+01))
    (Variables|Default|SetTimer _returnvalue)
    (Development|PrintString "Wave Timer Cleared")))

(fn ConstructionScript)

(fn GetGameDifficultyEnemyOffset
  (bind _asbp_body_friontline_game_instance (Utilities|Casting|CastToBP_BodyFriontlineGameInstance (Game|GetGameInstance)))
  (if (Utilities|Enum|Equal(Enum) (Variables|/Script/BodyFrontline.BodyFrontlineGameInstance|GetDiffculty _asbp_body_friontline_game_instance) "EGD_Hard")
    (return 2)
    (elif (Utilities|Enum|Equal(Enum) (Variables|/Script/BodyFrontline.BodyFrontlineGameInstance|GetDiffculty _asbp_body_friontline_game_instance) "EGD_Medium")
      (return 1)
      (elif (Utilities|Enum|Equal(Enum) (Variables|/Script/BodyFrontline.BodyFrontlineGameInstance|GetDiffculty _asbp_body_friontline_game_instance) "EGD_Easy")
        (return 0)))))

(fn GetBaseHealthEnemyOffset
  (params (BaseHealth :type Integer))
  (if (Math|Integer|InRange(Integer) BaseHealth 70 100)
    (Variables|Default|Setenemy_offset (+ (Variables|Default|Getenemy_offset) 2))
    (elif (Math|Integer|InRange(Integer) BaseHealth 30 70 true false)
      (Variables|Default|Setenemy_offset (+ (Variables|Default|Getenemy_offset) 1))))
  (Development|PrintString (Utilities|String|ToString(Integer) (+ (Variables|Default|GetDefault_Enemy) (Variables|Default|Getenemy_offset))) true true "(R=1.000000,G=0.918816,B=0.308330,A=1.000000)" 0.0)
  (return (+ (Variables|Default|GetDefault_Enemy) (Variables|Default|Getenemy_offset))))

(fn GetPlayerHealthEnemyOffset
  (params (Character :type BP%20White%20Blood%20Cell%20Character%20Object%20Reference))
  (bind _returnvalue (Class|WhiteBloodCellCharacter|HealthPercent Character))
  (if (>= _returnvalue 0.75)
    (return 1)
    (elif (Math|Float|InRange(Float) _returnvalue 0.4 0.75 false false)
      (return 0)
      (elif (<= _returnvalue 0.4)
        (return -1)))))

(fn GetProgressEnemyOffset
  (params (Character :type BP%20White%20Blood%20Cell%20Character%20Object%20Reference))
  (bind _returnvalue (Class|WhiteBloodCellCharacter|WaveNumber Character))
  (if (<= _returnvalue 3)
    (return 1)
    (elif (Math|Integer|InRange(Integer) _returnvalue 3 7 false false)
      (return 0)
      (elif (>= _returnvalue 7)
        (return -1)))))

(fn GetRBCEnemyOffset
  (params (Character :type BP%20White%20Blood%20Cell%20Character%20Object%20Reference))
  (bind _returnvalue (Class|WhiteBloodCellCharacter|RBCCount Character))
  (if (<= _returnvalue 2)
    (return -1)
    (elif (Math|Integer|InRange(Integer) _returnvalue 3 6)
      (return 0)
      (elif (>= _returnvalue 7)
        (return 2)))))

(fn SpawnEnemies
  (params (Amount :type Integer))
  (for _index (range 1 Amount)
    (Game|SpawnActorfromClass "/Game/Blueprints/Enemy/BP_Enemy.BP_Enemy_C" (Transformation|GetActorTransform) "Undefined" "MultiplyWithRoot" 0 0))
  (return))

(fn CalculateTimeEnemyOffset
  (params (Time :type Float%20%28double-precision%29))
  (if (Variables|Default|GetTimerStarted)
    (return 0)
    (elif (<= Time 3e+01)
      (return 2)
      (elif (Math|Float|InRange(Float) Time 3e+01 5e+01)
        (return 1)
        (elif (>= Time 5e+01)
          (return 0))))))